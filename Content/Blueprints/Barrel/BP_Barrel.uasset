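; BP_Barrel is a physics-driven barrel hazard that opens Lvl_FirstPerson when the first-person character overlaps its capsule.
; On BeginPlay it launches the Barrel component along the actor's forward vector, with a weaker velocity-change impulse for the Enemy variant than for the Normal one.
; Every Tick it adds a constant forward acceleration, independent of mass, to keep the barrel moving.
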(event OnComponentBeginOverlap(Capsule)
  (params (OverlappedComponent :type Primitive%20Component%20Object%20Reference) (OtherActor :type Actor%20Object%20Reference) (OtherComp :type Primitive%20Component%20Object%20Reference) (OtherBodyIndex :type Integer) (bFromSweep :type Boolean) (SweepResult :type Hit%20Result%20Structure%20%28by%20ref%29))
  (Utilities|Casting|CastToBP_FirstPersonCharacter OtherActor)
  (Game|OpenLevel(byName) "Lvl_FirstPerson"))

(event EventBeginPlay
  (switch Utilities|FlowControl|Switch|SwitchonE_BarrelType "NewEnumerator1"
    (:NewEnumerator0
      (Physics|AddImpulse (Variables|Default|GetBarrel) (* (Transformation|GetActorForwardVector) 5e+02) "None" true))
    (:NewEnumerator1
      (Physics|AddImpulse (Variables|Default|GetBarrel) (* (Transformation|GetActorForwardVector) 3e+03) "None" true))))

(event EventTick
  (params (DeltaSeconds :type Float%20%28single-precision%29))
  (Physics|AddForce (Variables|Default|GetBarrel) (* (Transformation|GetActorForwardVector) 1e+03) "None" true))

(fn ConstructionScript)